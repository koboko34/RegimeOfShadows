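; Player character Blueprint that handles pausing, music switching, the melee swing visual and an interact-prompt flag.
; HandlePause toggles game pause, reusing one pause menu widget and swapping input mode and cursor, or closes an open options submenu first.
; Music events forward calm and battle swaps to the cached BP_GameInstance.
; WeaponSwing uses a timeline to yaw MeleeAnchor through a turn scaled to -360 degrees.
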(event `self.ReceiveBeginPlay`
  (bind _asbp_game_instance (cast `/Game/Blueprints/BP_GameInstance` (`GameplayStatics.GetGameInstance`)))
  (set `self.BP Game Instance` _asbp_game_instance))

(event `self.HandlePause`
  (bind _returnvalue (`GameplayStatics.GetPlayerController` 0))
  (if (`GameplayStatics.IsGamePaused`)
    (`/Engine/EditorBlueprintResources/StandardMacros.IsValid` (`/Game/UI/WBP_PauseMenu.OptionsWidget` (`self.PauseWidget`))
      (:`Is Valid`
        (`/Game/UI/WBP_PauseMenu.DestroyOptionsWidget` (`self.PauseWidget`)))
      (:`Is Not Valid`
        (`WidgetBlueprintLibrary.SetInputMode_GameOnly` _returnvalue true)
        (set `PlayerController.bShowMouseCursor` false _returnvalue)
        (`Widget.RemoveFromParent` (`self.PauseWidget`))
        (`GameplayStatics.SetGamePaused` false)))
    (else
      (`GameplayStatics.SetGamePaused` true)
      (`/Engine/EditorBlueprintResources/StandardMacros.IsValid` (`self.PauseWidget`)
        (:`Is Valid`
          _)
        (:`Is Not Valid`
          (bind _returnvalue_2 (`|CreateWidget` "/Game/UI/WBP_PauseMenu.WBP_PauseMenu_C" _returnvalue))
          (bind _output_get (set `self.PauseWidget` _returnvalue_2))))
      (`UserWidget.AddToViewport` _output_get 0)
      (`WidgetBlueprintLibrary.SetInputMode_GameAndUIEx` _returnvalue _output_get "LockInFullscreen" false true)
      (set `PlayerController.bShowMouseCursor` true (`GameplayStatics.GetPlayerController` 0)))))

(event `self.PlayCalmMusic`
  (`/Game/Blueprints/BP_GameInstance.SwapToCalm` (`self.BP Game Instance`)))

(event `self.PlayBattleMusic`
  (`/Game/Blueprints/BP_GameInstance.SwapToBattle` (`self.BP Game Instance`)))

(event `self.WeaponSwing`
  (bind (_direction _progress) (`Timeline|WeaponSwingTimeline` :!via `PlayFromStart`)
    (:`Update`
      (`SceneComponent.K2_SetRelativeRotation` (`self.MeleeAnchor`) (`KismetMathLibrary.MakeRotator` 0.0 0.0 (* _progress -360.0)) false false))))

(fn `GetShowInteractPrompt`
  (returns (bShowInteractPrompt :type Boolean))
  (return (`self.bShowInteractPrompt`)))

(fn `HideInteractPrompt`
  (set `self.bShowInteractPrompt` false))

(fn `ShowInteractPrompt`
  (set `self.bShowInteractPrompt` true))

(fn `UserConstructionScript`)