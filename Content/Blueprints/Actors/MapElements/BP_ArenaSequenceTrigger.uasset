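; BP_ArenaSequenceTrigger is a one-shot overlap trigger that runs the dragon boss arena intro when the player enters.
; It hides the HUD and plays the sleep sequence, whose finish wakes the Dragon, starts the wake sequence and spawns BP_ArenaPostProcess.
; After the wake sequence's duration, it sets the current boss, restores input and HUD, then destroys itself.
; Without a valid sleep sequence, it jumps straight to that final handoff, skipping the wake-up.
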(event `self.ReceiveBeginPlay`
  (bind _asbp_player_controller (cast `/Game/Blueprints/Controllers/BP_PlayerController` (`GameplayStatics.GetPlayerController` 0)))
  (set `self.BP Player Controller` _asbp_player_controller))

(event `self.CollisionComponent.OnComponentBeginOverlap`
  (params (OverlappedComponent :type "PrimitiveComponent Object Reference") (OtherActor :type "Actor Object Reference") (OtherComp :type "PrimitiveComponent Object Reference") (OtherBodyIndex :type Integer) (bFromSweep :type Boolean) (SweepResult :type "HitResult Structure (by ref)"))
  (bind _arenasequencesleep (`self.ArenaSequenceSleep`))
  (bind _sequenceplayer (`LevelSequenceActor.SequencePlayer` _arenasequencesleep))
  (if (== OtherActor (`GameplayStatics.GetPlayerCharacter` 0))
    (`KismetSystemLibrary.Delay` 0.2)
    (`/Game/Blueprints/Controllers/BP_PlayerController.HideHUD` (`self.BP Player Controller`))
    (`/Engine/EditorBlueprintResources/StandardMacros.IsValid` _arenasequencesleep
      (:`Is Valid`
        (add `MovieSceneSequencePlayer.OnFinished` _sequenceplayer (delegate `OnFinished_Event`))
        (`MovieSceneSequencePlayer.Play` _sequenceplayer))
      (:`Is Not Valid`
        (bind _asplayer_character (cast `PlayerCharacter` (`GameplayStatics.GetPlayerCharacter` 0) :!label _label)
          (:`then`
            (`PlayerCharacter.SetCurrentBoss` _asplayer_character (`self.Dragon`)))
          (:`CastFailed`
            _))
        (`self.EnableInput` (`GameplayStatics.GetPlayerCharacter` 0) (`GameplayStatics.GetPlayerController` 0))
        (`/Game/Blueprints/Controllers/BP_PlayerController.ShowHUD` (`self.BP Player Controller`))
        (`self.K2_DestroyActor`)))))

(event `OnFinished_Event`
  (bind _sequenceplayer (`LevelSequenceActor.SequencePlayer` (`self.ArenaSequenceWake`)))
  (`/Game/Blueprints/Actors/Pawns/BP_Dragon.Wake Up` (`self.Dragon`))
  (`MovieSceneSequencePlayer.Play` _sequenceplayer)
  (`|SpawnActorFromClass` "/Game/Blueprints/Actors/MapElements/BP_ArenaPostProcess.BP_ArenaPostProcess_C" (`KismetMathLibrary.MakeTransform` (0.0 0.0 0.0)) "AlwaysSpawn" "MultiplyWithRoot" null null)
  (`KismetSystemLibrary.Delay` (`TimeManagementBlueprintLibrary.Conv_QualifiedFrameTimeToSeconds` (`MovieSceneSequencePlayer.GetDuration` _sequenceplayer)))
  (goto _label))

(fn `UserConstructionScript`)