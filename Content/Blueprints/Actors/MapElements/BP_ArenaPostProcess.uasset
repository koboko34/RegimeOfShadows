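; BP_ArenaPostProcess is a self-destroying arena actor that plays a temporary post-process effect when it spawns.
; On BeginPlay a timeline drives UpdatePostProcess with two tracks, then destroys the actor when it finishes.
; The Progress track scales chromatic aberration and vignette toward their configured maximums, while the GainAlpha track sets all four gain channels uniformly.
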(event `self.ReceiveBeginPlay`
  (bind (_direction _progress _gainalpha) (`Timeline|Timeline` :!via `PlayFromStart`)
    (:`Update`
      (`self.UpdatePostProcess` _progress _gainalpha))
    (:`Finished`
      (`self.K2_DestroyActor`))))

(fn `UpdatePostProcess`
  (params (Alpha :type "Float (double-precision)") (GainAlpha :type "Float (double-precision)"))
  (locals (`Chromatic Aberration Max` :type "Float (double-precision)" :default 5.0) (`Vignette Max` :type "Float (double-precision)" :default 1.0))
  (set `PostProcessComponent.Settings` (make `PostProcessSettings` :`ColorGain` (`KismetMathLibrary.MakeVector4` GainAlpha GainAlpha GainAlpha GainAlpha) :`SceneFringeIntensity` (* Alpha (`local.Chromatic Aberration Max`)) :`VignetteIntensity` (* Alpha (`local.Vignette Max`))) (`self.PostProcess`)))

(fn `UserConstructionScript`)