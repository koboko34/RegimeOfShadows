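; BP_Knight is an interactable map element whose mesh bobs and spins until the player uses it to spawn a BP_BonfireArena.
; A looping Timeline drives height and yaw offsets from the mesh's starting relative transform.
; PromptBox overlaps show and hide the player's interact prompt.
; Interact works once, spawning the arena at a hard-coded location and destroying the mesh, both boxes and spotlight, but not the actor.
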(event `self.ReceiveBeginPlay`
  (bind _starttransform (`self.StartTransform`))
  (bind _staticmesh (`self.StaticMesh`))
  (set `self.StartTransform` (`SceneComponent.GetRelativeTransform` (`self.StaticMesh`)))
  (bind (_direction _rotation _height) (`Timeline|Timeline` :!label _label)
    (:`Update`
      (`/Engine/EditorBlueprintResources/StandardMacros.IsValid` _staticmesh
        (:`Is Valid`
          (`SceneComponent.K2_SetRelativeLocationAndRotation` _staticmesh (`KismetMathLibrary.MakeVector` (.x (.location _starttransform)) (.y (.location _starttransform)) (+ (* _height (`self.HeightOffset`)) (.z (.location _starttransform)))) (`KismetMathLibrary.MakeRotator` (.roll (.rotation _starttransform)) (.pitch (.rotation _starttransform)) (+ _rotation (.yaw (.rotation _starttransform)))) false false))))
    (:`Finished`
      (goto _label :!via `PlayFromStart`))))

(event `InteractInterface.Interact`
  (`/Engine/EditorBlueprintResources/StandardMacros.DoOnce` false
    (:`Completed`
      (`|SpawnActorFromClass` "/Game/Blueprints/Actors/MapElements/BP_BonfireArena.BP_BonfireArena_C" (`KismetMathLibrary.MakeTransform` (34.0 -342.0 150.0)) "AlwaysSpawn" "MultiplyWithRoot" null null)
      (`ActorComponent.K2_DestroyComponent` (`self.StaticMesh`))
      (`ActorComponent.K2_DestroyComponent` (`self.InteractBox`))
      (`ActorComponent.K2_DestroyComponent` (`self.PromptBox`))
      (`ActorComponent.K2_DestroyComponent` (`self.SpotLight`)))))

(event `self.PromptBox.OnComponentBeginOverlap`
  (params (OverlappedComponent :type "PrimitiveComponent Object Reference") (OtherActor :type "Actor Object Reference") (OtherComp :type "PrimitiveComponent Object Reference") (OtherBodyIndex :type Integer) (bFromSweep :type Boolean) (SweepResult :type "HitResult Structure (by ref)"))
  (if (== OtherActor (`GameplayStatics.GetPlayerCharacter` 0))
    (bind _asbp_player_character (cast `/Game/Blueprints/Actors/BP_PlayerCharacter` OtherActor))
    (`/Game/Blueprints/Actors/BP_PlayerCharacter.ShowInteractPrompt` _asbp_player_character)))

(event `self.PromptBox.OnComponentEndOverlap`
  (params (OverlappedComponent :type "PrimitiveComponent Object Reference") (OtherActor :type "Actor Object Reference") (OtherComp :type "PrimitiveComponent Object Reference") (OtherBodyIndex :type Integer))
  (if (== OtherActor (`GameplayStatics.GetPlayerCharacter` 0))
    (bind _asbp_player_character (cast `/Game/Blueprints/Actors/BP_PlayerCharacter` OtherActor))
    (`/Game/Blueprints/Actors/BP_PlayerCharacter.HideInteractPrompt` _asbp_player_character)))

(fn `UserConstructionScript`)