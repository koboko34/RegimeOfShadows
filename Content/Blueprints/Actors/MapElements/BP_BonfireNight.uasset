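; BP_BonfireNight is an interactable map element that sends the player into the Arena level.
; Interacting disables player input, saves the PlayerCharacter's stats, then plays a timeline transition before opening the level.
; Each timeline update rebuilds the post-process settings, scaling chromatic aberration and vignette toward their maximums while a separate curve drives color gain.
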(event `InteractInterface.Interact`
  (bind _returnvalue (`GameplayStatics.GetPlayerCharacter` 0))
  (`self.DisableInput` _returnvalue (`GameplayStatics.GetPlayerController` 0))
  (bind _asplayer_character (cast `PlayerCharacter` _returnvalue))
  (`PlayerCharacter.SavePlayerStats` _asplayer_character)
  (bind (_direction _progress _gainalpha) (`Timeline|Timeline` :!via `PlayFromStart`)
    (:`Update`
      (`self.UpdatePostProcess` _progress _gainalpha))
    (:`Finished`
      (`GameplayStatics.OpenLevelBySoftObjectPtr` "/Game/Maps/Arena.Arena"))))

(fn `UpdatePostProcess`
  (params (Alpha :type "Float (double-precision)") (GainAlpha :type "Float (double-precision)"))
  (locals (`Chromatic Aberration Max` :type "Float (double-precision)" :default 5.0) (`Vignette Max` :type "Float (double-precision)" :default 1.0))
  (set `PostProcessComponent.Settings` (make `PostProcessSettings` :`ColorGain` (`KismetMathLibrary.MakeVector4` GainAlpha GainAlpha GainAlpha GainAlpha) :`SceneFringeIntensity` (* Alpha (`local.Chromatic Aberration Max`)) :`VignetteIntensity` (* Alpha (`local.Vignette Max`))) (`self.PostProcess`)))

(fn `UserConstructionScript`
  (`parent.UserConstructionScript`))