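; Enemy Blueprint that adds a floating health bar, elemental status visuals and random attack animation selection.
; Tick shows the world-space bar only on living, damaged non-boss enemies, updating its fill and turning it to face the player camera.
; Status events swap the mesh overlay material for burning, wet, frost or charged, or clear it.
; The construction script copies the hearing range into the PawnSensing hearing threshold.
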(event `self.ReceiveBeginPlay`
  (if (`self.bIsBoss`)
    (`SceneComponent.SetVisibility` (`self.Healthbar Widget`) false false)
    (else
      (bind _aswbp_health_bar (cast `/Game/UI/WBP_HealthBar` (`WidgetComponent.GetWidget` (`self.Healthbar Widget`))))
      (set `self.WBP Health Bar` _aswbp_health_bar))))

(event `self.ReceiveTick`
  (params (DeltaSeconds :type "Float (single-precision)"))
  (bind _healthbar_widget (`self.Healthbar Widget`))
  (bind _healthbar_widget_2 (`self.Healthbar Widget`))
  (if (`self.GetIsAlive`)
    (if (`self.bIsBoss`)
      _
      (elif (== (`self.GetMaxHealth`) (`self.GetHealth`))
        (`SceneComponent.SetVisibility` _healthbar_widget false false)
        (else
          (`SceneComponent.SetVisibility` _healthbar_widget true false)
          (bind _aswbp_health_bar (cast `/Game/UI/WBP_HealthBar` (`WidgetComponent.GetWidget` _healthbar_widget)))
          (`ProgressBar.SetPercent` (`/Game/UI/WBP_HealthBar.HealthBar` _aswbp_health_bar) (/ (`KismetMathLibrary.Conv_IntToDouble` (`self.GetHealth`)) (`KismetMathLibrary.Conv_IntToDouble` (`self.GetMaxHealth`))))
          (`SceneComponent.K2_SetWorldRotation` _healthbar_widget_2 (`KismetMathLibrary.FindLookAtRotation` (`SceneComponent.K2_GetComponentLocation` _healthbar_widget_2) (`SceneComponent.K2_GetComponentLocation` (`PlayerCameraManager.TransformComponent` (`GameplayStatics.GetPlayerCameraManager` 0)))) false false))))
    (else
      (`SceneComponent.SetVisibility` (`self.Healthbar Widget`) false false))))

(event `self.ApplyBurningMaterial`
  (`MeshComponent.SetOverlayMaterial` (`self.Mesh`) (`self.BurningMaterial`)))

(event `self.ApplyWetMaterial`
  (`MeshComponent.SetOverlayMaterial` (`self.Mesh`) (`self.WetMaterial`)))

(event `self.ApplyFrostMaterial`
  (`MeshComponent.SetOverlayMaterial` (`self.Mesh`) (`self.FrostMaterial`)))

(event `self.ApplyChargedMaterial`
  (`MeshComponent.SetOverlayMaterial` (`self.Mesh`) (`self.ChargedMaterial`)))

(event `self.RemoveStatusMaterial`
  (`MeshComponent.SetOverlayMaterial` (`self.Mesh`) null))

(fn `GetAttackAnimation`
  (returns (Anim :type "AnimMontage Object Reference"))
  (return (`KismetArrayLibrary.Array_Random` (`self.AttackAnimations`))))

(fn `UserConstructionScript`
  (set `PawnSensingComponent.HearingThreshold` (`self.GetHearingRange`) (`self.PawnSensingComponent`)))