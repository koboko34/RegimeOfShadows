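; BP_ZombieGirl is a zombie enemy pawn that can melee-attack the player.
; On begin play it sets its health to maximum.
; Its Attack event sphere-traces for pawns forward from an AttackPoint component over AttackRange, with debug drawing enabled.
; The first hit, if it casts to PlayerCharacter, takes Strength-based damage.
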(event `self.ReceiveBeginPlay`
  (`self.SetHealth` (`self.GetMaxHealth`)))

(event `/Game/Blueprints/Actors/Interfaces/BPI_ZombieAttacks.Attack`
  (bind _returnvalue (`SceneComponent.K2_GetComponentLocation` (`self.AttackPoint`)))
  (bind _outhits (`KismetSystemLibrary.SphereTraceMultiForObjects` :`Start` _returnvalue :`End` (+ _returnvalue (* (`self.GetActorForwardVector`) (`self.AttackRange`))) :`Radius` 75.0 :`ObjectTypes` (`|MakeArray` (enumliteral `EObjectTypeQuery` "ObjectTypeQuery3")) :`DrawDebugType` "ForDuration"))
  (for _array_element _outhits
    (bind _asplayer_character (cast `PlayerCharacter` (`.HitActor` (`GameplayStatics.BreakHitResult` _array_element))))
    (`GameplayStatics.ApplyDamage` _asplayer_character (`KismetMathLibrary.Conv_IntToDouble` (`self.GetStrength`)) (`self.GetController`) self "/Script/Engine.DamageType")
    (break)))

(fn `UserConstructionScript`)