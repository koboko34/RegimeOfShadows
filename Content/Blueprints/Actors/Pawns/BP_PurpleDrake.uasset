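; BP_PurpleDrake is a drake pawn that damages the player with mouth, claw and flamethrower attacks, starting at max health.
; Mouth and claw events sphere-trace pawns from mesh sockets, with debug drawing, dealing Strength-based damage (reduced for claws).
; Flamethrower start and end events toggle particles and an active flag.
; While active, the flame collider's begin-overlap deals Intelligence-based damage, limited to one player hit per activation.
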(event `self.ReceiveBeginPlay`
  (`parent.ReceiveBeginPlay`)
  (`self.SetHealth` (`self.GetMaxHealth`)))

(event `/Game/Blueprints/Actors/Interfaces/BPI_DragonAttacks.MouthAttack`
  (bind _returnvalue (`SceneComponent.GetSocketLocation` (`self.Mesh`) "MouthAttackSocket"))
  ;[1 1 1] Mouth Attack
  (bind _outhits (`KismetSystemLibrary.SphereTraceMultiForObjects` :`Start` _returnvalue :`End` (+ _returnvalue (* (`self.GetActorForwardVector`) 50.0)) :`Radius` 100.0 :`ObjectTypes` (`|MakeArray` (enumliteral `EObjectTypeQuery` "ObjectTypeQuery3")) :`DrawDebugType` "ForDuration"))
  (for _array_element _outhits
    (bind _asplayer_character (cast `PlayerCharacter` (`.HitActor` (`GameplayStatics.BreakHitResult` _array_element))))
    (`GameplayStatics.ApplyDamage` _asplayer_character (`KismetMathLibrary.Conv_IntToDouble` (`self.GetStrength`)) (`self.GetController`) self "/Script/Engine.DamageType")
    (break)))

(event `/Game/Blueprints/Actors/Interfaces/BPI_DragonAttacks.ClawAttack`
  (bind _mesh (`self.Mesh`))
  (bind _returnvalue (* (`self.GetActorForwardVector`) 50.0))
  ;[1 1 1] Claw Attack
  (bind _outhits (`KismetSystemLibrary.SphereTraceMultiForObjects` :`Start` (+ (`SceneComponent.GetSocketLocation` _mesh "ClawAttackSocket_L") _returnvalue) :`End` (+ _returnvalue (`SceneComponent.GetSocketLocation` _mesh "ClawAttackSocket_R")) :`Radius` 100.0 :`ObjectTypes` (`|MakeArray` (enumliteral `EObjectTypeQuery` "ObjectTypeQuery3")) :`DrawDebugType` "ForDuration"))
  (for _array_element _outhits
    (bind _asplayer_character (cast `PlayerCharacter` (`.HitActor` (`GameplayStatics.BreakHitResult` _array_element))))
    (`GameplayStatics.ApplyDamage` _asplayer_character (* (`self.GetStrength`) 0.6) (`self.GetController`) self "/Script/Engine.DamageType")
    (break)))

(event `/Game/Blueprints/Actors/Interfaces/BPI_DragonAttacks.StartFlamethrower`
  ;[1 1 1] Flamethrower
  (`ActorComponent.Activate` (`self.FlamethrowerParticles`) false)
  (set `self.FlamethrowerActive` true)
  (set `self.RecentlyHitPlayer` false))

(event `/Game/Blueprints/Actors/Interfaces/BPI_DragonAttacks.EndFlamethrower`
  ;[1 1 1] Flamethrower
  (`ActorComponent.Deactivate` (`self.FlamethrowerParticles`))
  (set `self.FlamethrowerActive` false)
  (set `self.RecentlyHitPlayer` false))

(event `self.FlamethrowerCollider.OnComponentBeginOverlap`
  (params (OverlappedComponent :type "PrimitiveComponent Object Reference") (OtherActor :type "Actor Object Reference") (OtherComp :type "PrimitiveComponent Object Reference") (OtherBodyIndex :type Integer) (bFromSweep :type Boolean) (SweepResult :type "HitResult Structure (by ref)"))
  ;[1 1 1] Flamethrower
  (if (and (`self.FlamethrowerActive`) (not (`self.RecentlyHitPlayer`)))
    (bind _asbp_player_character (cast `/Game/Blueprints/Actors/BP_PlayerCharacter` OtherActor))
    (`GameplayStatics.ApplyDamage` _asbp_player_character (`KismetMathLibrary.Conv_IntToDouble` (`self.GetIntelligence`)) (`self.GetController`) self)
    (set `self.RecentlyHitPlayer` true)))

(fn `UserConstructionScript`
  (`parent.UserConstructionScript`))