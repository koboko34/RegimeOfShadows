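; Dragon boss pawn that wakes with a scream, fights with flamethrower, jump and mouth attacks, and summons a Purple Drake as second boss.
; Flamethrower and jump use flag-gated overlap colliders limited to one hit per activation; the bite sphere-traces at a mouth socket, with damage scaled from stats.
; Waking sets the AI blackboard, summoning also heals the dragon, and GetAttackAnimation makes a weighted random pick.
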(event `Wake Up`
  (`self.WakeUp`))

(event `self.ReceiveBeginPlay`
  (`parent.ReceiveBeginPlay`)
  (`self.SetHealth` (`self.GetMaxHealth`)))

(event `/Game/Blueprints/Actors/Interfaces/BPI_DragonAttacks.StartFlamethrower`
  ;[1 1 1] Flamethrower
  (`ActorComponent.Activate` (`self.FlamethrowerParticles`) false)
  (set `self.FlamethrowerActive` true)
  (set `self.RecentlyHitPlayer` false))

(event `/Game/Blueprints/Actors/Interfaces/BPI_DragonAttacks.EndFlamethrower`
  ;[1 1 1] Flamethrower
  (`ActorComponent.Deactivate` (`self.FlamethrowerParticles`))
  (set `self.FlamethrowerActive` false)
  (set `self.RecentlyHitPlayer` false))

(event `self.FlamethrowerCollider.OnComponentBeginOverlap`
  (params (OverlappedComponent :type "PrimitiveComponent Object Reference") (OtherActor :type "Actor Object Reference") (OtherComp :type "PrimitiveComponent Object Reference") (OtherBodyIndex :type Integer) (bFromSweep :type Boolean) (SweepResult :type "HitResult Structure (by ref)"))
  ;[1 1 1] Flamethrower
  (if (and (`self.FlamethrowerActive`) (not (`self.RecentlyHitPlayer`)))
    (bind _asbp_player_character (cast `/Game/Blueprints/Actors/BP_PlayerCharacter` OtherActor))
    (`GameplayStatics.ApplyDamage` _asbp_player_character (`KismetMathLibrary.Conv_IntToDouble` (`self.GetIntelligence`)) (`self.GetController`) self)
    (set `self.RecentlyHitPlayer` true)))

(event `/Game/Blueprints/Actors/Interfaces/BPI_DragonAttacks.StartJumpAttack`
  ;[1 1 1] Jump Attack
  (set `self.JumpAttackActive` true)
  (set `self.RecentlyHitPlayer` false))

(event `/Game/Blueprints/Actors/Interfaces/BPI_DragonAttacks.EndJumpAttack`
  ;[1 1 1] Jump Attack
  (set `self.JumpAttackActive` false)
  (set `self.RecentlyHitPlayer` false))

(event `self.JumpAttackCollider.OnComponentBeginOverlap`
  (params (OverlappedComponent :type "PrimitiveComponent Object Reference") (OtherActor :type "Actor Object Reference") (OtherComp :type "PrimitiveComponent Object Reference") (OtherBodyIndex :type Integer) (bFromSweep :type Boolean) (SweepResult :type "HitResult Structure (by ref)"))
  ;[1 1 1] Jump Attack
  (if (and (`self.JumpAttackActive`) (not (`self.RecentlyHitPlayer`)))
    (bind _asbp_player_character (cast `/Game/Blueprints/Actors/BP_PlayerCharacter` OtherActor))
    (`GameplayStatics.ApplyDamage` _asbp_player_character (* (`self.GetStrength`) 1.2) (`self.GetController`) self)
    (set `self.RecentlyHitPlayer` true)))

(event `/Game/Blueprints/Actors/Interfaces/BPI_DragonAttacks.MouthAttack`
  (bind _returnvalue (`SceneComponent.GetSocketLocation` (`self.Mesh`) "MouthAttackSocket"))
  ;[1 1 1] Mouth Attack
  (bind _outhits (`KismetSystemLibrary.SphereTraceMultiForObjects` :`Start` _returnvalue :`End` _returnvalue :`Radius` 75.0 :`ObjectTypes` (`|MakeArray` (enumliteral `EObjectTypeQuery` "ObjectTypeQuery3")) :`DrawDebugType` "ForDuration"))
  (for _array_element _outhits
    (bind _asplayer_character (cast `PlayerCharacter` (`.HitActor` (`GameplayStatics.BreakHitResult` _array_element))))
    (`GameplayStatics.ApplyDamage` _asplayer_character (`KismetMathLibrary.Conv_IntToDouble` (`self.GetStrength`)) (`self.GetController`) self "/Script/Engine.DamageType")
    (break)))

(event `/Game/Blueprints/Actors/Interfaces/BPI_DragonAttacks.SummonDrake`
  (bind _returnvalue (`self.GetMaxHealth`))
  ;[1 1 1] Summon Purple Drake
  (if (`self.GetIsAwake`)
    (`self.SetHealth` (`KismetMathLibrary.Min` (+ (`self.GetHealth`) (* _returnvalue (`self.ScreamHeal`))) _returnvalue))
    (`KismetSystemLibrary.Delay` 2.0)
    (`KismetSystemLibrary.PrintString` "Summon drake called")
    (bind _returnvalue_2 (`|SpawnActorFromClass` "/Game/Blueprints/Actors/Pawns/BP_PurpleDrake.BP_PurpleDrake_C" (`KismetMathLibrary.MakeTransform` (+ (`self.K2_GetActorLocation`) (0.0 0.0 1000.0))) "AdjustIfPossibleButAlwaysSpawn" "MultiplyWithRoot" null self))
    (bind _asbp_player_character (cast `/Game/Blueprints/Actors/BP_PlayerCharacter` (`GameplayStatics.GetPlayerCharacter` 0)))
    (`PlayerCharacter.SetCurrentBossTwo` _asbp_player_character _returnvalue_2)))

(event `/Game/Blueprints/Actors/Interfaces/BPI_DragonAttacks.PlayScreamSound`
  (`GameplayStatics.PlaySoundAtLocation` "/Game/Sounds/DragonRoar_Cue.DragonRoar_Cue" (`self.K2_GetActorLocation`) (struct) (`self.RoarVolume`) 1.0 0.0 null null null null)
  (`/Game/Blueprints/Actors/Interfaces/BPI_DragonAttacks.EndFlamethrower`))

(fn `GetAttackAnimation`
  (returns (Anim :type "AnimMontage Object Reference"))
  (bind _attackanimations (`self.AttackAnimations`))
  (switch `int` (`KismetMathLibrary.RandomIntegerInRange` 0 9)
    (:`0`
      _)
    (:`1`
      _)
    (:`2`
      _)
    (:`3`
      (return (`|GetArrayItem` _attackanimations 1)))
    (:`4`
      (return (`|GetArrayItem` _attackanimations 1)))
    (:`5`
      (return (`|GetArrayItem` _attackanimations 1)))
    (:`6`
      (return (`|GetArrayItem` _attackanimations 1)))
    (:`7`
      (return (`|GetArrayItem` _attackanimations 1)))
    (:`8`
      (return (`|GetArrayItem` _attackanimations 2)))
    (:`9`
      (return (`|GetArrayItem` _attackanimations 2))))
  (return (`|GetArrayItem` _attackanimations)))

(fn `UserConstructionScript`
  (`parent.UserConstructionScript`))